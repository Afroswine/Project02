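; Blueprint function library of material helpers, with a single function, SetMaterialEmission, that recolors a mesh and sets its emissive glow at runtime.
; It creates a dynamic material instance from the mesh's slot 0 material, then sets its base color, emissive color and emissive multiplier parameters from the inputs.
; Each call creates the instance from the current material on that slot, and only the first slot is affected.
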(fn `SetMaterialEmission`
  (params (StaticMesh :type "PrimitiveComponent Object Reference") (BaseColor :type "LinearColor Structure" :default (struct :`R` 1.0 :`B` 1.0 :`A` 1.0)) (EmissiveColor :type "LinearColor Structure" :default (struct :`R` 1.0 :`B` 1.0 :`A` 1.0)) (EmissiveMultiplier :type "Float (double-precision)" :default 1.0))
  (locals (materialInstance :type "MaterialInstanceDynamic Object Reference"))
  (bind _returnvalue (`PrimitiveComponent.CreateDynamicMaterialInstance` StaticMesh 0 (`PrimitiveComponent.GetMaterial` StaticMesh 0) "DynamicMaterialInstance"))
  (bind _output_get (set `local.materialInstance` _returnvalue))
  (`MaterialInstanceDynamic.SetVectorParameterValue` _output_get "Base Color" (`local.BaseColor`))
  (`MaterialInstanceDynamic.SetScalarParameterValue` (`local.materialInstance`) "Emissive Multiplier" (`local.EmissiveMultiplier`))
  (`MaterialInstanceDynamic.SetVectorParameterValue` (`local.materialInstance`) "Emissive Color" (`local.EmissiveColor`)))