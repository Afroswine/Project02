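; BP_Door is an interactable door that swings open away from the player and closes on the next interaction.
; An ACInteract component shows and hides the prompt widget through OnShowUI and OnHideUI; the box overlap logic is disabled.
; OnInteract alternates playing and reversing a timeline that lerps mesh yaw toward an angle signed by a forward-vector dot product.
; Mesh collision and further interaction are blocked until the animation finishes.
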(event `/Game/CustomMechanics/Interfaces/BI_Interactable.OnShowUI`
  (params (isSelected :type Boolean))
  ;[1 1 1] UI Widget Display
  (`/Game/CustomMechanics/Blueprints/Components/AC_Interact.ShowUI` (`self.AC_Interact`) isSelected))

(event `self.ReceiveBeginPlay`
  ;[1 1 1] Event BeginPlay
  (`/Game/CustomMechanics/Blueprints/Components/AC_Interact.SetWidget` (`self.AC_Interact`) (`self.Widget_InteractPrompt`)))

(event `/Game/CustomMechanics/Interfaces/BI_Interactable.OnHideUI`
  ;[1 1 1] UI Widget Display
  (`/Game/CustomMechanics/Blueprints/Components/AC_Interact.HideUI` (`self.AC_Interact`)))

(event `/Game/CustomMechanics/Interfaces/BI_Interactable.OnInteract`
  ;[1 1 1] On Interact - Disable physics collisions and animate the door opening/closing away from the player
  (if (not (`self.IsAnimating`))
    (set `self.IsAnimating` true)
    (`PrimitiveComponent.SetCollisionEnabled` (`self.DoorMesh`) "NoCollision")
    (`/Engine/EditorBlueprintResources/StandardMacros.FlipFlop`
      (:`A`
        (`self.SetDoorOpenAngle`)
        (bind (_direction _door_track) (`Timeline|Open/Close Door Timeline` :!label _label)
          (:`Update`
            (`SceneComponent.K2_SetRelativeRotation` (`self.DoorMesh`) (`KismetMathLibrary.MakeRotator` 0.0 0.0 (`KismetMathLibrary.Lerp` 0.0 (`self.DoorOpenAngle`) _door_track)) false false))
          (:`Finished`
            (`PrimitiveComponent.SetCollisionEnabled` (`self.DoorMesh`) "QueryAndPhysics")
            (set `self.IsAnimating` false))))
      (:`B`
        (goto _label :!via `Reverse`)))))

(fn `SetDoorOpenAngle`
  ;[1 1 1] Determine which way the door should open based on the player's position relative to the door...
  (set `self.DoorOpenAngle` (`KismetMathLibrary.SelectFloat` -110.0 110.0 (>= (`KismetMathLibrary.Dot_VectorVector` (`self.GetActorForwardVector`) (`KismetMathLibrary.GetDirectionUnitVector` (`self.K2_GetActorLocation`) (`self.K2_GetActorLocation` (`GameplayStatics.GetPlayerPawn` 0)))) 0.0)))
  (return))

(fn `UserConstructionScript`)