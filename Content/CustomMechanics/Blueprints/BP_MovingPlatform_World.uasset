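; BP_MovingPlatform_World is a moving platform whose timeline is meant to lerp it in world space from its start to an end-reference mesh's location over Duration.
; Player or pickup overlaps (if TriggeredByPlayer) and pressure switch counts play the timeline forward, or reverse it when released.
; Overlapping pickups snap-attach to PickupPoint.
; The construction script applies PlatformMesh to both platform and end reference.
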(event `self.ReceiveBeginPlay`
  ;[1 1 1] EventBeginPlay - Set start location
  (`|ExecutionSequence`
    (:`then_0`
      (set `self.startLocation` (`SceneComponent.K2_GetComponentLocation` (`self.PlatformMain`)))
      (set `self.EndLocation` (`SceneComponent.K2_GetComponentLocation` (`self.PlatformEndReference`))))))

(event `self.Box.OnComponentBeginOverlap`
  (params (OverlappedComponent :type "PrimitiveComponent Object Reference") (OtherActor :type "Actor Object Reference") (OtherComp :type "PrimitiveComponent Object Reference") (OtherBodyIndex :type Integer) (bFromSweep :type Boolean) (SweepResult :type "HitResult Structure (by ref)"))
  ;[1 1 1] Triggers - Collisions
  (`self.AddCollidingActors` OtherActor)
  (if (> (`KismetArrayLibrary.Array_Length` (`self.collidingActors`)) 0)
    (`self.PlayTimeline` false)))

(event `self.Box.OnComponentEndOverlap`
  (params (OverlappedComponent :type "PrimitiveComponent Object Reference") (OtherActor :type "Actor Object Reference") (OtherComp :type "PrimitiveComponent Object Reference") (OtherBodyIndex :type Integer))
  ;[1 1 1] Triggers - Collisions
  (for _array_element (`self.collidingActors`)
    (if (== _array_element OtherActor)
      (`KismetArrayLibrary.Array_RemoveItem` (`self.collidingActors`) _array_element)))
  (if (and (== (`KismetArrayLibrary.Array_Length` (`self.collidingActors`)) 0) (or (< (`self.PressureSwitchesActive`) (`self.PressureSwitchesNeeded`)) (== (`self.PressureSwitchesActive`) 0)))
    (`self.PlayTimeline` true)))

(event `SwitchActivated`
  ;[1 1 1] Triggers - PressureSwitches
  (bind _result (`/Engine/EditorBlueprintResources/StandardMacros.IncrementInt` (`self.PressureSwitchesActive`))
    (:`  `
      (`self.PlayTimeline` (not (>= _result (`self.PressureSwitchesNeeded`)))))))

(event `SwitchDeactivated`
  ;[1 1 1] Triggers - PressureSwitches
  (`|ExecutionSequence`
    (:`then_0`
      (if (> (`self.PressureSwitchesActive`) 0)
        (`/Engine/EditorBlueprintResources/StandardMacros.DecrementInt` (`self.PressureSwitchesActive`))))
    (:`then_1`
      (`self.PlayTimeline` (or (< (`self.PressureSwitchesActive`) (`self.PressureSwitchesNeeded`)) (== (`self.PressureSwitchesActive`) 0))))))

(fn `AddCollidingActors`
  (params (otherActor :type "Actor Object Reference"))
  (locals (collidingActor :type "Actor Object Reference"))
  (set `local.collidingActor` otherActor)
  (if (`self.TriggeredByPlayer`)
    (`|ExecutionSequence`
      (:`then_0`
        (bind _asbp_third_person_character (cast `/Game/ThirdPerson/Blueprints/BP_ThirdPersonCharacter` (`local.collidingActor`)))
        (`KismetArrayLibrary.Array_AddUnique` (`self.collidingActors`) _asbp_third_person_character)
        (return))
      (:`then_1`
        (bind _asbp_pickup (cast `/Game/CustomMechanics/Blueprints/BP_Pickup` (`local.collidingActor`)))
        (`KismetArrayLibrary.Array_AddUnique` (`self.collidingActors`) _asbp_pickup)
        (`self.K2_AttachToComponent` _asbp_pickup (`self.PickupPoint`) "None" "SnapToTarget" "SnapToTarget" "KeepWorld" true)
        (return)))))

(fn `PlayTimeline`
  (params (isReversed :type Boolean))
  (`TimelineComponent.SetPlayRate` (`self.PlatformTimeline`) (/ 1.0 (`self.Duration`)))
  (if isReversed
    (`TimelineComponent.Reverse` (`self.PlatformTimeline`))
    (else
      (`TimelineComponent.Play` (`self.PlatformTimeline`)))))

(fn `UserConstructionScript`
  (`StaticMeshComponent.SetStaticMesh` (`self.PlatformMain`) (`self.platformMesh`))
  (`StaticMeshComponent.SetStaticMesh` (`self.PlatformEndReference`) (`self.platformMesh`)))