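; BP_PressureSwitch is a pressure plate that activates or deactivates linked PlatformsToActivate when actors overlap it.
; An overlap box tracks occupants, so only the first arrival and last departure matter, and a timeline animates the switch.
; Togglers keep their state on release, while normal switches flip back.
; The construction script sets initial state and materials from IsDeactivator and IsToggler; older activation logic remains unconnected in the event graph.
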(event `self.OverlapBox.OnComponentBeginOverlap`
  (params (OverlappedComponent :type "PrimitiveComponent Object Reference") (OtherActor :type "Actor Object Reference") (OtherComp :type "PrimitiveComponent Object Reference") (OtherBodyIndex :type Integer) (bFromSweep :type Boolean) (SweepResult :type "HitResult Structure (by ref)"))
  ;[1 1 1] Collisions - Inform PlatformToActivate of activation status
  (`KismetArrayLibrary.Array_AddUnique` (`self.collidingActors`) OtherActor)
  (if (== 1 (`KismetArrayLibrary.Array_Length` (`self.collidingActors`)))
    (`self.ActivateOrDeactivate`)))

(event `self.OverlapBox.OnComponentEndOverlap`
  (params (OverlappedComponent :type "PrimitiveComponent Object Reference") (OtherActor :type "Actor Object Reference") (OtherComp :type "PrimitiveComponent Object Reference") (OtherBodyIndex :type Integer))
  ;[1 1 1] Collisions - Inform PlatformToActivate of activation status
  (`KismetArrayLibrary.Array_RemoveItem` (`self.collidingActors`) OtherActor)
  (if (== 0 (`KismetArrayLibrary.Array_Length` (`self.collidingActors`)))
    (if (`self.IsToggler`)
      (`TimelineComponent.Reverse` (`self.SwitchTimeline`))
      (else
        (`self.ActivateOrDeactivate`)
        (`TimelineComponent.Reverse` (`self.SwitchTimeline`))))))

(fn `ActivateOrDeactivate`
  (locals (NewLocalVar :type String))
  (if (`self.isActive`)
    (for _array_element (`self.PlatformsToActivate`)
      (`/Game/CustomMechanics/Blueprints/BP_MovingPlatform.SwitchDeactivated` _array_element))
    (else
      (for _array_element_2 (`self.PlatformsToActivate`)
        (`/Game/CustomMechanics/Blueprints/BP_MovingPlatform.SwitchActivated` _array_element_2))))
  (`TimelineComponent.Play` (`self.SwitchTimeline`))
  (bind _output_get (set `self.isActive` (not (`self.isActive`))))
  (`KismetSystemLibrary.PrintString` (`KismetStringLibrary.Concat_StrStr` "isActive: " (`KismetStringLibrary.Conv_BoolToString` _output_get))))

(fn `ToggleSwitchMaterial`
  (if (`self.isActive`)
    (`PrimitiveComponent.SetMaterial` (`self.Switch`) 0 "/Game/LevelPrototyping/Materials/MI_Solid_Orange.MI_Solid_Orange")
    (else
      (`PrimitiveComponent.SetMaterial` (`self.Switch`) 0 "/Game/LevelPrototyping/Materials/MI_Solid_Green.MI_Solid_Green"))))

(fn `UserConstructionScript`
  (if (`self.IsDeactivator`)
    (set `self.isActive` true)
    (else
      (set `self.isActive` false)))
  (`self.ToggleSwitchMaterial`)
  (if (`self.IsToggler`)
    (`PrimitiveComponent.SetMaterial` (`self.Base`) 0 "/Game/LevelPrototyping/Materials/MI_Solid_Black.MI_Solid_Black")))