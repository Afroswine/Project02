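; AC_Interact is an actor component that manages an in-world interaction prompt for its owning actor.
; SetWidget stores a WidgetComponent and casts its widget to Widget_InteractPrompt for later calls.
; ShowUI updates the prompt's text and color from the selection state and unhides the component, while HideUI hides it.
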(event `SetWidget`
  (params (`Widget Component` :type "WidgetComponent Object Reference"))
  ;[1 1 1] SetWidget - Set widget variables (Should be called on 'Event Begin Play')
  (bind _output_get (set `self.widgetComponent` `Widget Component`))
  (bind _aswidget_interact_prompt (cast `/Game/CustomMechanics/Blueprints/UI/Widget_InteractPrompt` (`WidgetComponent.GetWidget` _output_get)))
  (set `self.widgetInteract` _aswidget_interact_prompt))

(event `ShowUI`
  (params (isSelected :type Boolean))
  ;[1 1 1] ShowUI - Set text and color based on 'isSelected' and unhide 'widgetComponent'
  (`/Game/CustomMechanics/Blueprints/UI/Widget_InteractPrompt.SetTextAndColor` (`self.widgetInteract`) isSelected)
  (`SceneComponent.SetHiddenInGame` (`self.widgetComponent`) false false))

(event `HideUI`
  ;[1 1 1] HideUI - Set 'widgetComponent' to Hidden
  (`SceneComponent.SetHiddenInGame` (`self.widgetComponent`) true false))