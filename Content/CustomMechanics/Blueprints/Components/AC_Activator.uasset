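; AC_Activator is a component that switches a list of target objects on and off.
; ActivateObjects and DeactivateObjects send the matching interface message to each entry in ObjectsToActivate and update the Active flag.
; ToggleObjects picks between the two based on that flag.
; With IsDeactivator set, Active starts true on BeginPlay without messaging the targets, so the first toggle deactivates them.
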(event `self.ReceiveBeginPlay`
  (if (`self.isDeactivator`)
    (set `self.active` true)))

(fn `ActivateObjects`
  (for _array_element (`self.objectsToActivate`)
    (message `/Game/CustomMechanics/Interfaces/BI_Activatable.Activate` (`KismetSystemLibrary.Conv_InterfaceToObject` _array_element)))
  (set `self.active` true))

(fn `DeactivateObjects`
  (for _array_element (`self.objectsToActivate`)
    (message `/Game/CustomMechanics/Interfaces/BI_Activatable.Deactivate` (`KismetSystemLibrary.Conv_InterfaceToObject` _array_element)))
  (set `self.active` false))

(fn `ToggleObjects`
  (if (`self.active`)
    (`self.DeactivateObjects`)
    (else
      (`self.ActivateObjects`))))