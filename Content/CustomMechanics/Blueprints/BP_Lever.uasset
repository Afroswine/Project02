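; BP_Lever is an interactable lever that toggles objects through its ACActivator component.
; ACInteract handles showing and hiding the prompt widget.
; Each interaction plays or reverses a timeline that pitches the lever, flipping direction when it finishes, then toggles the objects and updates the head material to match the activator's active state.
; The construction script picks the initial head material from the activator's IsDeactivator flag.
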(event `/Game/CustomMechanics/Interfaces/BI_Interactable.OnShowUI`
  (params (isSelected :type Boolean))
  ;[1 1 1] Show/Hide Widget
  (`/Game/CustomMechanics/Blueprints/Components/AC_Interact.ShowUI` (`self.AC_Interact`) isSelected))

(event `self.ReceiveBeginPlay`
  ;[1 1 1] Set Widget
  (`/Game/CustomMechanics/Blueprints/Components/AC_Interact.SetWidget` (`self.AC_Interact`) (`self.Widget`)))

(event `/Game/CustomMechanics/Interfaces/BI_Interactable.OnHideUI`
  ;[1 1 1] Show/Hide Widget
  (`/Game/CustomMechanics/Blueprints/Components/AC_Interact.HideUI` (`self.AC_Interact`)))

(event `/Game/CustomMechanics/Interfaces/BI_Interactable.OnInteract`
  ;[1 1 1] Interact - Activate Objects and provide feedback
  (if (`self.timelineForward`)
    (`TimelineComponent.Play` (`self.AnimationTimeline`))
    (else
      (`TimelineComponent.Reverse` (`self.AnimationTimeline`))))
  (`/Game/CustomMechanics/Blueprints/Components/AC_Activator.ToggleObjects` (`self.AC_Activator`))
  (`self.ToggleMaterial`))

(fn `ToggleMaterial`
  (if (`/Game/CustomMechanics/Blueprints/Components/AC_Activator.active` (`self.AC_Activator`))
    (`PrimitiveComponent.SetMaterial` (`self.Head`) 0 (`self.ActiveMaterial`))
    (else
      (`PrimitiveComponent.SetMaterial` (`self.Head`) 0 (`self.InactiveMaterial`)))))

(fn `UserConstructionScript`
  (if (`/Game/CustomMechanics/Blueprints/Components/AC_Activator.isDeactivator` (`self.AC_Activator`))
    (`PrimitiveComponent.SetMaterial` (`self.Head`) 0 (`self.ActiveMaterial`))
    (else
      (`PrimitiveComponent.SetMaterial` (`self.Head`) 0 (`self.InactiveMaterial`)))))