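; BP_AudioTrigger is a trigger volume that plays an assigned ambient audio source when the player pawn enters it.
; The Box overlap event checks for player pawn 0, waits AudioDelayTimer through a retriggerable delay, then plays the audio component of AmbientAudioToPlay from the start.
; If no audio source is assigned, it prints an on-screen warning instead.
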(event `self.Box.OnComponentBeginOverlap`
  (params (OverlappedComponent :type "PrimitiveComponent Object Reference") (OtherActor :type "Actor Object Reference") (OtherComp :type "PrimitiveComponent Object Reference") (OtherBodyIndex :type Integer) (bFromSweep :type Boolean) (SweepResult :type "HitResult Structure (by ref)"))
  (if (== OtherActor (`GameplayStatics.GetPlayerPawn` 0))
    (`/Engine/EditorBlueprintResources/StandardMacros.IsValid` (`self.AmbientAudioToPlay`) ; If AmbientAudioToPlay has been set...
      (:`Is Valid`
        (`KismetSystemLibrary.RetriggerableDelay` (`self.AudioDelayTimer`)) ; Wait this long...
        (`AudioComponent.Play` (`AmbientSound.AudioComponent` (`self.AmbientAudioToPlay`)) 0.0) ; Play the specified audio source
      )
      (:`Is Not Valid`
        (`KismetSystemLibrary.PrintString` "AmbientAudioToPlay has not been set on a BP_AudioTrigger")))))

(fn `UserConstructionScript`)