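; BP_FallingPlatform is a platform that moves from its start to an end location when its Box is overlapped.
; Overlaps gather characters and pickups into CollidingActors and play the timeline, which reverses when an exit leaves that list empty.
; PlatformTimeline lerps PlatformMain's relative location at a rate set by Duration.
; The construction script applies mesh, scale and rotation to the platform and an end-position reference mesh.
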(event `self.ReceiveBeginPlay`
  ;[1 1 1] EventBeginPlay - Set start location
  (set `self.startLocation` (`SceneComponent.RelativeLocation` (`self.PlatformMain`))))

(event `self.Box.OnComponentBeginOverlap`
  (params (OverlappedComponent :type "PrimitiveComponent Object Reference") (OtherActor :type "Actor Object Reference") (OtherComp :type "PrimitiveComponent Object Reference") (OtherBodyIndex :type Integer) (bFromSweep :type Boolean) (SweepResult :type "HitResult Structure (by ref)"))
  ;[1 1 1] Collisions
  (`self.AddCollidingActors` OtherActor OtherComp)
  (`self.PlayTimeline` false))

(event `self.Box.OnComponentEndOverlap`
  (params (OverlappedComponent :type "PrimitiveComponent Object Reference") (OtherActor :type "Actor Object Reference") (OtherComp :type "PrimitiveComponent Object Reference") (OtherBodyIndex :type Integer))
  ;[1 1 1] Collisions
  (for _array_element (`self.collidingActors`)
    (if (== _array_element OtherActor)
      (`KismetArrayLibrary.Array_RemoveItem` (`self.collidingActors`) _array_element)))
  (if (== (`KismetArrayLibrary.Array_Length` (`self.collidingActors`)) 0)
    (`self.PlayTimeline` true)))

(fn `AddCollidingActors`
  (params (otherActor :type "Actor Object Reference") (otherComp :type "PrimitiveComponent Object Reference"))
  (locals (collidingActor :type "Actor Object Reference") (collidingComp :type "PrimitiveComponent Object Reference"))
  (`|ExecutionSequence`
    (:`then_0`
      (for _array_element (`self.GetOverlappingActors` "/Script/Engine.Actor")
        (bind _asbp_third_person_character (cast `/Game/ThirdPerson/Blueprints/BP_ThirdPersonCharacter` _array_element))
        (`KismetArrayLibrary.Array_Add` (`self.collidingActors`) _asbp_third_person_character)))
    (:`then_1`
      (for _array_element_2 (`self.GetOverlappingActors` "/Script/Engine.Actor")
        (bind _asbp_pickup (cast `/Game/CustomMechanics/Blueprints/BP_Pickup` _array_element_2))
        (if (== (`/Game/CustomMechanics/Blueprints/BP_Pickup.StaticMesh` _asbp_pickup) (`local.collidingComp`))
          (`KismetArrayLibrary.Array_Add` (`self.collidingActors`) _asbp_pickup))))))

(fn `PlayTimeline`
  (params (isReversed :type Boolean))
  (`TimelineComponent.SetPlayRate` (`self.PlatformTimeline`) (/ 1.0 (`self.Duration`)))
  (if isReversed
    (`TimelineComponent.Reverse` (`self.PlatformTimeline`))
    (else
      (`TimelineComponent.Play` (`self.PlatformTimeline`)))))

(fn `UserConstructionScript`
  (bind _platformmain (`self.PlatformMain`))
  (bind _platformendreference (`self.PlatformEndReference`))
  (bind _platformmesh (`self.platformMesh`))
  (`StaticMeshComponent.SetStaticMesh` _platformmain _platformmesh)
  (`StaticMeshComponent.SetStaticMesh` _platformendreference _platformmesh)
  (`SceneComponent.SetRelativeScale3D` _platformmain (`self.Scale`))
  (`SceneComponent.SetRelativeScale3D` _platformendreference (`self.Scale`))
  (`SceneComponent.K2_SetRelativeRotation` _platformmain (`self.Rotation`) false false)
  (`SceneComponent.K2_SetRelativeRotation` _platformendreference (`self.Rotation`) false false)
  (`SceneComponent.K2_SetRelativeLocation` _platformendreference (`self.EndLocation`) false false))