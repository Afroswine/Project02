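; BP_Door is an interactable door that toggles on interaction and shows a prompt widget.
; On BeginPlay it hands its mesh and timeline to ACDoor and its widget to ACInteract, which handles showing and hiding the prompt.
; Interaction calls ToggleDoor unless the door is animating.
; The timeline has no wired play input in this graph; its Update and Finished outputs forward to ACDoor.
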(event `/Game/MyAssets/Code/Blueprints/Interactable/Interfaces/BI_Interactable.OnShowUI`
  (params (isSelected :type Boolean))
  ;[1 1 1] UI Widget Display
  (`/Game/MyAssets/Code/Blueprints/Interactable/Components/AC_Interact.ShowUI` (`self.AC_Interact`) isSelected))

(event `self.ReceiveBeginPlay`
  ;[1 1 1] Event BeginPlay
  (`/Game/MyAssets/Code/Blueprints/Interactable/Components/AC_Door.Setup` (`self.AC_Door`) (`self.DoorMesh`) (`self.DoorTimeline`))
  (`/Game/MyAssets/Code/Blueprints/Interactable/Components/AC_Interact.SetWidget` (`self.AC_Interact`) (`self.Widget_InteractPrompt`)))

(event `/Game/MyAssets/Code/Blueprints/Interactable/Interfaces/BI_Interactable.OnHideUI`
  ;[1 1 1] UI Widget Display
  (`/Game/MyAssets/Code/Blueprints/Interactable/Components/AC_Interact.HideUI` (`self.AC_Interact`)))

(event `/Game/MyAssets/Code/Blueprints/Interactable/Interfaces/BI_Interactable.OnInteract`
  ;[1 1 1] On Interact
  (if (not (`/Game/MyAssets/Code/Blueprints/Interactable/Components/AC_Door.isAnimating` (`self.AC_Door`)))
    (`/Game/MyAssets/Code/Blueprints/Interactable/Components/AC_Door.ToggleDoor` (`self.AC_Door`))))

(fn `UserConstructionScript`)