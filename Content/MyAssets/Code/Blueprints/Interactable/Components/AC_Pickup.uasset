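; Pickup component that lets its owning actor be attached to a socket on a new parent and dropped back as a physics object.
; Setup caches the supplied mesh, its offset, its children and the owner's root.
; Pickup disables physics, snaps the owner to the socket and restores the mesh offset.
; BeginPlay and Drop enable physics and rebuild the cached attachment hierarchy, with Drop also zeroing velocity and detaching the owner.
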(event `self.ReceiveBeginPlay`
  (`PrimitiveComponent.SetSimulatePhysics` (`self.pickupMesh`) true)
  (`self.SetHierarchy`))

(fn `Drop`
  (`|ExecutionSequence`
    (:`then_0`
      (`PrimitiveComponent.SetSimulatePhysics` (`self.pickupMesh`) true)
      (`self.SetHierarchy`)
      (`PrimitiveComponent.SetAllPhysicsLinearVelocity` (`self.pickupMesh`) (0.0 0.0 0.0) false))
    (:`then_1`
      (`Actor.K2_DetachFromActor` (`self.owner`) "KeepWorld" "KeepWorld" "KeepWorld"))))

(fn `Pickup`
  (params (NewParent :type "SceneComponent Object Reference") (SocketName :type Name))
  (`PrimitiveComponent.SetSimulatePhysics` (`self.pickupMesh`) false)
  (`Actor.K2_AttachToComponent` (`self.owner`) (`local.NewParent`) (`local.SocketName`) "SnapToTarget" "SnapToTarget" "KeepWorld" true)
  (`SceneComponent.K2_SetRelativeLocation` (`self.pickupMesh`) (`self.pickupMeshOffset`) false false))

(fn `SetHierarchy`
  (for _array_element (`self.childrenOfPickupMesh`)
    (`SceneComponent.K2_AttachToComponent` _array_element (`self.pickupMesh`) "None" "SnapToTarget" "SnapToTarget" "KeepWorld" true))
  (`SceneComponent.K2_AttachToComponent` (`self.pickupMesh`) (`self.root`) "None" "SnapToTarget" "SnapToTarget" "KeepWorld" true))

(fn `Setup`
  (params (`Mesh Component` :type "StaticMeshComponent Object Reference"))
  (set `self.pickupMesh` `Mesh Component`)
  (bind _output_get (set `self.owner` (`self.GetOwner`)))
  (set `self.root` (`Actor.RootComponent` _output_get))
  (set `self.pickupMeshOffset` (`SceneComponent.RelativeLocation` (`self.pickupMesh`)))
  (set `self.childrenOfPickupMesh` (`SceneComponent.GetChildrenComponents` (`self.pickupMesh`) true)))