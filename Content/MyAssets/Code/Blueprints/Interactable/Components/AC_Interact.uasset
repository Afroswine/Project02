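; AC_Interact is an actor component that manages an animated interaction prompt for interactable objects.
; SetWidget caches the owner's widget component and its WBP_InteractPrompt, hides it and records a Z range just above its starting height.
; ShowUI reveals the prompt with text and color based on selection state, and HideUI hides it.
; Tick continuously bobs the widget with a timed linear ping-pong lerp, even while hidden.
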(event `SetWidget`
  (params (`Widget Component` :type "WidgetComponent Object Reference"))
  (bind (_relativelocation_x _relativelocation_y _relativelocation_z) (`KismetMathLibrary.BreakVector` (`SceneComponent.RelativeLocation` (`self.widgetComponent`))))
  ;[1 1 1] SetWidget - Set widget variables (Should be called on 'Event Begin Play')
  (bind _output_get (set `self.widgetComponent` `Widget Component`))
  (bind _aswbp_interact_prompt (cast `/Game/MyAssets/Code/Blueprints/Interactable/UI/WBP_InteractPrompt` (`WidgetComponent.GetWidget` _output_get)))
  (set `self.widgetInteract` _aswbp_interact_prompt)
  (`SceneComponent.SetHiddenInGame` (`self.widgetComponent`) true false)
  (bind _output_get_2 (set `self.startZ` _relativelocation_z))
  (set `self.endZ` (+ _output_get_2 10.0)))

(event `ShowUI`
  (params (isSelected :type Boolean))
  ;[1 1 1] ShowUI - Set text and color based on 'isSelected' and unhide 'widgetComponent'
  (`/Game/MyAssets/Code/Blueprints/Interactable/UI/WBP_InteractPrompt.SetTextAndColor` (`self.widgetInteract`) isSelected)
  (`SceneComponent.SetHiddenInGame` (`self.widgetComponent`) false false))

(event `HideUI`
  ;[1 1 1] HideUI - Set 'widgetComponent' to Hidden
  (`SceneComponent.SetHiddenInGame` (`self.widgetComponent`) true false))

(event `self.ReceiveTick`
  (params (DeltaSeconds :type "Float (single-precision)"))
  ;[1 1 1] Animate Widget
  (bind _output_get (set `self.currentTime` (+ DeltaSeconds (`self.currentTime`))))
  (if (< _output_get (`self.endTime`))
    (if (`self.lerpForward`)
      (set `self.currentZ` (`KismetMathLibrary.Lerp` (`self.startZ`) (`self.endZ`) (/ (`self.currentTime`) (`self.endTime`))))
      (else
        (set `self.currentZ` (`KismetMathLibrary.Lerp` (`self.endZ`) (`self.startZ`) (/ (`self.currentTime`) (`self.endTime`))))))
    (`SceneComponent.K2_SetRelativeLocation` (`self.widgetComponent`) (`KismetMathLibrary.MakeVector` 0.0 0.0 (`self.currentZ`)) false false)
    (else
      (set `self.currentTime` 0.0)
      (set `self.lerpForward` (not (`self.lerpForward`))))))