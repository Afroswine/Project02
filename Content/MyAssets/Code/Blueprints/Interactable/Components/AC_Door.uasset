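; Actor component that opens and closes a door by rotating a mesh around yaw, using a mesh and timeline passed in through Setup.
; ToggleDoor plays or reverses the timeline, whose update lerps the yaw toward the open angle.
; When opening, it can pick the angle's sign from a dot product so the door swings away from the player.
; Collision can be disabled during animation and is restored when the timeline finishes.
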(fn `OnTimelineFinished`
  (`PrimitiveComponent.SetCollisionEnabled` (`self.doorMesh`) "QueryAndPhysics")
  (set `self.isAnimating` false))

(fn `OnTimelineUpdate`
  (params (track :type "Float (double-precision)"))
  (`SceneComponent.K2_SetRelativeRotation` (`self.doorMesh`) (`KismetMathLibrary.MakeRotator` 0.0 0.0 (`KismetMathLibrary.Lerp` 0.0 (`self.RelativeAngle`) track)) false false))

(fn `SetDoorOpenDirection`
  (set `self.RelativeAngle` (`KismetMathLibrary.SelectFloat` (* (`self.DoorOpenAngle`) -1.0) (`self.DoorOpenAngle`) (>= (`KismetMathLibrary.Dot_VectorVector` (`Actor.GetActorForwardVector` (`self.GetOwner`)) (`KismetMathLibrary.GetDirectionUnitVector` (`Actor.K2_GetActorLocation` (`self.GetOwner`)) (`Actor.K2_GetActorLocation` (`GameplayStatics.GetPlayerPawn` 0)))) 0.0))))

(fn `Setup`
  (params (doorMesh :type "StaticMeshComponent Object Reference") (doorTimeline :type "TimelineComponent Object Reference"))
  (set `self.doorMesh` doorMesh)
  (set `self.timeline` doorTimeline)
  (set `self.RelativeAngle` (`self.DoorOpenAngle`)))

(fn `ToggleDoor`
  (`|ExecutionSequence`
    (:`then_0`
      (if (`self.disableCollisionWhileAnimating`)
        (`PrimitiveComponent.SetCollisionEnabled` (`self.doorMesh`) "NoCollision")))
    (:`then_1`
      (set `self.isAnimating` true)
      (if (`self.toggle`)
        (if (`self.openAwayFromPlayer`)
          (`self.SetDoorOpenDirection`))
        (`TimelineComponent.Play` (`self.timeline`))
        (else
          (`TimelineComponent.Reverse` (`self.timeline`))))
      (set `self.toggle` (not (`self.toggle`))))))