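; AC_Activator is a component that lets interactable actors activate, deactivate or toggle a list of linked actors.
; On BeginPlay it gathers AC_Activatable components from ActivatableActors, warning about any missing one, and later calls their switch functions while playing a matching sound.
; Setup creates an emissive material instance for ChangeColor to blend from inactive to active, using orange when IsDeactivator starts it activated and green otherwise.
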(event `self.ReceiveBeginPlay`
  (`|ExecutionSequence`
    (:`then_0`
      (if (`self.isDeactivator`)
        (set `self.isActivated` true)))
    (:`then_1`
      (for (_array_element _array_index) (`self.activatableActors`)
        (bind _returnvalue (`Actor.GetComponentByClass` _array_element "/Game/MyAssets/Code/Blueprints/Interactable/Components/AC_Activatable.AC_Activatable_C"))
        (if (`KismetSystemLibrary.IsValid` _returnvalue)
          (`KismetArrayLibrary.Array_AddUnique` (`self.activatables`) _returnvalue)
          (else
            (`KismetSystemLibrary.PrintString` (`KismetStringLibrary.Concat_StrStr` "WARNING: " (`KismetSystemLibrary.GetDisplayName` (`self.GetOwner`)) " contains an item at 'activatableActors[" (`KismetStringLibrary.Conv_IntToString` _array_index) " ]' that does not have an 'AC_Activatable' component!") true true (struct :`R` 1.0 :`B` 0.5 :`A` 1.0) 10.0)))))))

(fn `ActivateObjects`
  (for _array_element (`self.activatables`)
    (`/Game/MyAssets/Code/Blueprints/Interactable/Components/AC_Activatable.SwitchActivated` _array_element))
  (set `self.isActivated` true)
  (`self.PlaySoundActivated`))

(fn `ChangeColor`
  (params (alpha :type "Float (double-precision)"))
  (bind _returnvalue (`KismetMathLibrary.LinearColorLerp` (`self.colorInactive`) (`self.colorActive`) (`local.alpha`)))
  (`/Game/MyAssets/Code/Materials/BFL_Materials.SetMaterialEmissive` (`self.materialInstance`) _returnvalue _returnvalue (`KismetMathLibrary.Lerp` (`self.emissionInactive`) (`self.emissionActivate`) (`local.alpha`))))

(fn `DeactivateObjects`
  (for _array_element (`self.activatables`)
    (`/Game/MyAssets/Code/Blueprints/Interactable/Components/AC_Activatable.SwitchDeactivated` _array_element))
  (set `self.isActivated` false)
  (`self.PlaySoundDeactivated`))

(fn `PlaySoundActivated`
  (if (`KismetSystemLibrary.IsValid` (`self.audioComponent`))
    (`AudioComponent.SetSound` (`self.audioComponent`) (`self.clipActivated`))
    (`AudioComponent.Play` (`self.audioComponent`) 0.0)
    (else
      (`KismetSystemLibrary.PrintString` (`KismetStringLibrary.Concat_StrStr` (`KismetSystemLibrary.GetObjectName` (`self.GetOwner`)) ": No AudioComponent Set.") true true (struct :`R` 1.0 :`B` 1.0 :`A` 1.0)))))

(fn `PlaySoundDeactivated`
  (if (`KismetSystemLibrary.IsValid` (`self.audioComponent`))
    (`AudioComponent.SetSound` (`self.audioComponent`) (`self.clipDeactivated`))
    (`AudioComponent.Play` (`self.audioComponent`) 0.0)
    (else
      (`KismetSystemLibrary.PrintString` (`KismetStringLibrary.Concat_StrStr` (`KismetSystemLibrary.GetObjectName` (`self.GetOwner`)) ": No AudioComponent Set.") true true (struct :`R` 1.0 :`B` 1.0 :`A` 1.0)))))

(fn `Setup`
  (params (emissiveMesh :type "StaticMeshComponent Object Reference") (audioComp :type "AudioComponent Object Reference"))
  (bind _colorinactive (`self.colorInactive`))
  (`|ExecutionSequence`
    (:`then_0`
      (if (`self.isDeactivator`)
        (set `self.isActivated` true)))
    (:`then_1`
      (bind _materialinstance (`/Game/MyAssets/Code/Materials/BFL_Materials.CreateMaterialInstanceFromMesh` (`local.emissiveMesh`)))
      (set `self.materialInstance` _materialinstance)
      (if (`KismetSystemLibrary.IsValid` (`local.audioComp`))
        (set `self.audioComponent` (`local.audioComp`))))
    (:`then_2`
      (if (`self.isDeactivator`)
        (set `self.colorInactive` (struct :`R` 0.2 :`G` 0.07451 :`A` 1.0))
        (set `self.colorActive` (struct :`R` 1.0 :`G` 0.501961 :`A` 1.0))
        (set `self.isActivated` true)
        (else
          (set `self.colorInactive` (struct :`G` 0.070588 :`A` 1.0))
          (set `self.colorActive` (struct :`G` 1.0 :`A` 1.0))))
      (`/Game/MyAssets/Code/Materials/BFL_Materials.SetMaterialEmissive` (`self.materialInstance`) _colorinactive _colorinactive (`self.emissionInactive`)))))

(fn `ToggleObjects`
  (if (`self.isActivated`)
    (`self.DeactivateObjects`)
    (else
      (`self.ActivateObjects`))))