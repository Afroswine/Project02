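; BP_Gate is an interactable two-door gate that opens and closes in response to switch activation.
; On BeginPlay, it gives each door component its mesh and timeline, then binds to the activatable component's activated and deactivated events.
; Activation plays both timelines and deactivation reverses them.
; Each timeline forwards its update value and finished event to its door component, which handles the door's response.
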(event `self.ReceiveBeginPlay`
  ;[1 1 1] EventBeginPlay
  (`|ExecutionSequence`
    (:`then_0`
      (`/Game/MyAssets/Code/Blueprints/Interactable/Components/AC_Door.Setup` (`self.AC_DoorA`) (`self.Gate_DoorA`) (`self.DoorA_Timeline`))
      (`/Game/MyAssets/Code/Blueprints/Interactable/Components/AC_Door.Setup` (`self.AC_DoorB`) (`self.Gate_DoorB`) (`self.DoorB_Timeline`)))
    (:`then_1`
      (add `/Game/MyAssets/Code/Blueprints/Interactable/Components/AC_Activatable.OnSwitchActivated` (`self.AC_Activatable`) (delegate `OnSwitchActivated`)))
    (:`then_2`
      (add `/Game/MyAssets/Code/Blueprints/Interactable/Components/AC_Activatable.OnSwitchDeactivated` (`self.AC_Activatable`) (delegate `OnSwitchDeactivated`)))))

(event `OnSwitchActivated`
  ;[1 1 1] EventBeginPlay
  (`TimelineComponent.Play` (`self.DoorA_Timeline`))
  (`TimelineComponent.Play` (`self.DoorB_Timeline`)))

(event `OnSwitchDeactivated`
  ;[1 1 1] EventBeginPlay
  (`TimelineComponent.Reverse` (`self.DoorA_Timeline`))
  (`TimelineComponent.Reverse` (`self.DoorB_Timeline`)))

(fn `UserConstructionScript`)