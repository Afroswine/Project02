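; BP_PressureSwitch is a pressure plate that switches linked objects on while any actor overlaps its box and off once all have left.
; It tracks overlapping actors in a unique list, so only the first arrival and last departure trigger ACActivator to toggle the objects.
; Those transitions play or reverse a timeline that moves the switch vertically and drives its emissive color through the same activator component.
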(event `self.ReceiveBeginPlay`
  ;[1 1 1] Begin Play
  (`/Game/MyAssets/Code/Blueprints/Interactable/Components/AC_Activator.Setup` (`self.AC_Activator`) (`self.Switch`) (`self.AudioSource`)))

(event `self.OverlapBox.OnComponentBeginOverlap`
  (params (OverlappedComponent :type "PrimitiveComponent Object Reference") (OtherActor :type "Actor Object Reference") (OtherComp :type "PrimitiveComponent Object Reference") (OtherBodyIndex :type Integer) (bFromSweep :type Boolean) (SweepResult :type "HitResult Structure (by ref)"))
  ;[1 1 1] Collisions - Inform PlatformToActivate of activation status
  (`KismetArrayLibrary.Array_AddUnique` (`self.collidingActors`) OtherActor)
  (if (== 1 (`KismetArrayLibrary.Array_Length` (`self.collidingActors`)))
    (`/Game/MyAssets/Code/Blueprints/Interactable/Components/AC_Activator.ToggleObjects` (`self.AC_Activator`) true)
    (`TimelineComponent.Play` (`self.SwitchTimeline`))))

(event `self.OverlapBox.OnComponentEndOverlap`
  (params (OverlappedComponent :type "PrimitiveComponent Object Reference") (OtherActor :type "Actor Object Reference") (OtherComp :type "PrimitiveComponent Object Reference") (OtherBodyIndex :type Integer))
  ;[1 1 1] Collisions - Inform PlatformToActivate of activation status
  (`KismetArrayLibrary.Array_RemoveItem` (`self.collidingActors`) OtherActor)
  (if (== 0 (`KismetArrayLibrary.Array_Length` (`self.collidingActors`)))
    (`/Game/MyAssets/Code/Blueprints/Interactable/Components/AC_Activator.ToggleObjects` (`self.AC_Activator`) false)
    (`TimelineComponent.Reverse` (`self.SwitchTimeline`))))

(fn `UserConstructionScript`)