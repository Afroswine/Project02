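; Actor component that tracks how many switches currently activate its owner, for interactables driven by one or more switches.
; Switch activated and deactivated events raise or lower an active count and each fire a matching dispatcher.
; GetIsActive reports whether that count meets or exceeds the required number of switches.
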(event `SwitchActivated`
  (`/Engine/EditorBlueprintResources/StandardMacros.IncrementInt` (`self.switchesActive`)
    (:`  `
      (`self.OnSwitchActivated`))))

(event `SwitchDeactivated`
  (`/Engine/EditorBlueprintResources/StandardMacros.DecrementInt` (`self.switchesActive`)
    (:`  `
      (`self.OnSwitchDeactivated`))))

(fn `GetIsActive`
  (returns (isActive :type Boolean))
  (return (>= (`self.switchesActive`) (`self.switchesNeeded`))))