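; Interactable lever that toggles linked objects through its ACActivator component each time the player uses it.
; ACInteract handles showing and hiding the prompt widget, while ACActivator is set up with the head mesh and audio component for feedback.
; A timeline pitches the lever and drives the color change, alternating forward and reverse, with interaction ignored while it plays.
; Objects toggle as the animation starts, without waiting for it to finish.
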(event `/Game/MyAssets/Code/Interactable/Interfaces/BI_Interactable.OnShowUI`
  (params (isSelected :type Boolean))
  ;[1 1 1] Show/Hide Widget
  (`/Game/MyAssets/Code/Interactable/Components/AC_Interact.ShowUI` (`self.AC_Interact`) isSelected))

(event `self.ReceiveBeginPlay`
  ;[1 1 1] Begin Play
  (`/Game/MyAssets/Code/Interactable/Components/AC_Activator.Setup` (`self.AC_Activator`) (`self.Head`) (`self.Audio`))
  (`/Game/MyAssets/Code/Interactable/Components/AC_Interact.SetWidget` (`self.AC_Interact`) (`self.Widget`)))

(event `/Game/MyAssets/Code/Interactable/Interfaces/BI_Interactable.OnHideUI`
  ;[1 1 1] Show/Hide Widget
  (`/Game/MyAssets/Code/Interactable/Components/AC_Interact.HideUI` (`self.AC_Interact`)))

(event `/Game/MyAssets/Code/Interactable/Interfaces/BI_Interactable.OnInteract`
  ;[1 1 1] Interact - Activate Objects and provide feedback
  (if (not (`self.timelinePlaying`))
    (if (`self.timelineForward`)
      (`TimelineComponent.Play` (`self.AnimationTimeline`))
      (else
        (`TimelineComponent.Reverse` (`self.AnimationTimeline`))))
    (set `self.timelinePlaying` true)
    (`/Game/MyAssets/Code/Interactable/Components/AC_Activator.ToggleObjects` (`self.AC_Activator`))))

(fn `UserConstructionScript`)